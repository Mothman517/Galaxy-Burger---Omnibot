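; BP_Corpse is an animal corpse that the player hunter can harvest.
; On BeginPlay it caches the player and configures its HarvestableComponent with resource, harvested state and destroy-on-harvest setting.
; A sphere overlap sets or clears that component as the player's ClosestHarvestable, printing debug text.
; Each tick the sprite turns on yaw only to face the player, acting as a billboard.
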(event OnComponentBeginOverlap(Sphere)
  (params (OverlappedComponent :type Primitive%20Component%20Object%20Reference) (OtherActor :type Actor%20Object%20Reference) (OtherComp :type Primitive%20Component%20Object%20Reference) (OtherBodyIndex :type Integer) (bFromSweep :type Boolean) (SweepResult :type Hit%20Result%20Structure%20%28by%20ref%29))
  ;[0.15 0.15 0.15 0.5] Collision Detection Toggles
  (if (Actor|ActorHasTag OtherActor "Player")
    (Variables|/Game/PlayerControllers/Hunter/Blueprints/BP_PlayerHunter.BP_PlayerHunter_C|SetClosest%20Harvestable (Variables|Default|GetPlayerRef) (Variables|Default|GetHarvestableComponent))
    (Development|PrintString "IN")))

(event OnComponentEndOverlap(Sphere)
  (params (OverlappedComponent :type Primitive%20Component%20Object%20Reference) (OtherActor :type Actor%20Object%20Reference) (OtherComp :type Primitive%20Component%20Object%20Reference) (OtherBodyIndex :type Integer))
  ;[0.15 0.15 0.15 0.5] Collision Detection Toggles
  (if (Actor|ActorHasTag OtherActor "Player")
    (Variables|/Game/PlayerControllers/Hunter/Blueprints/BP_PlayerHunter.BP_PlayerHunter_C|SetClosest%20Harvestable (Variables|Default|GetPlayerRef) 0)
    (Development|PrintString "OUT")))

(event EventBeginPlay
  (bind _harvestablecomponent (Variables|Default|GetHarvestableComponent))
  ;[0.15 0.15 0.15 0.5] Set Player Ref
  (bind _asbp_player_hunter (Utilities|Casting|CastToBP_PlayerHunter (Game|GetPlayerCharacter 0)))
  (Variables|Default|SetPlayerRef _asbp_player_hunter)
  (Default|SetVariables _harvestablecomponent (Variables|/Game/Entities/Components/HarvestableComponent.HarvestableComponent_C|GetObtainableResource _harvestablecomponent) (Variables|Default|GetHas%20Been%20Harvested) (Variables|Default|GetDestoryOnHarvest)))

(event EventTick
  (params (DeltaSeconds :type Float%20%28single-precision%29))
  ;[0.15 0.15 0.15 0.5] Billboard Sprite
  (Transformation|SetWorldRotation (Variables|Default|GetSprite) (Math|Rotator|MakeRotator 0.0 0.0 (+ (.Yaw (Math|Rotator|BreakRotator (Math|Rotator|FindLookatRotation (Transformation|GetWorldLocation (Variables|Collision|GetCapsuleComponent)) (Transformation|GetWorldLocation (Variables|/Script/Engine.Character|GetCapsuleComponent (Game|GetPlayerCharacter 0)))))) -9e+01)) false false))

(fn ConstructionScript)