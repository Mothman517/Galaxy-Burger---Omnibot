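; Base food pickup that displays an ingredient sprite (cheese, buns or beef) and registers itself with the player when in range.
; GetSprite maps IngredientType to a sprite, applied on BeginPlay and whenever UpdateFoodSprite changes the type.
; Billboarding is a one-time yaw rotation at BeginPlay, derived from the player's CamPosition and capsule location.
; Sphere overlaps with Player-tagged actors toggle IsOverlapping and set or clear the player's ClosestPickup, without comparing distances.
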(event OnComponentBeginOverlap(Sphere1)
  (params (OverlappedComponent :type Primitive%20Component%20Object%20Reference) (OtherActor :type Actor%20Object%20Reference) (OtherComp :type Primitive%20Component%20Object%20Reference) (OtherBodyIndex :type Integer) (bFromSweep :type Boolean) (SweepResult :type Hit%20Result%20Structure%20%28by%20ref%29))
  ;[0.15 0.15 0.15 0.5] Collision Detection Toggles
  (if (Actor|ActorHasTag OtherActor "Player")
    (Variables|Default|SetisOverlapping true)
    (Variables|/Game/PlayerControllers/Chef/Blueprints/BP_ThirdPersonCharacter.BP_ThirdPersonCharacter_C|SetclosestPickup (Variables|Default|GetPlayerRef) self)))

(event OnComponentEndOverlap(Sphere1)
  (params (OverlappedComponent :type Primitive%20Component%20Object%20Reference) (OtherActor :type Actor%20Object%20Reference) (OtherComp :type Primitive%20Component%20Object%20Reference) (OtherBodyIndex :type Integer))
  ;[0.15 0.15 0.15 0.5] Collision Detection Toggles
  (if (Actor|ActorHasTag OtherActor "Player")
    (Variables|Default|SetisOverlapping false)
    (Variables|/Game/PlayerControllers/Chef/Blueprints/BP_ThirdPersonCharacter.BP_ThirdPersonCharacter_C|SetclosestPickup (Variables|Default|GetPlayerRef) 0)))

(event EventBeginPlay
  (bind _returnvalue (Game|GetPlayerCharacter 0))
  ;[0.15 0.15 0.15 0.5] Setting the sprite + Billboarding
  (bind _newparam (CallFunction|GetSprite))
  (Rendering|Components|Sprite|SetSprite (Variables|Default|GetSprite) _newparam)
  (bind _asbp_third_person_character (Utilities|Casting|CastToBP_ThirdPersonCharacter _returnvalue))
  (bind _output_get (Variables|Default|SetPlayerRef _asbp_third_person_character))
  (Transformation|SetWorldRotation (Variables|Default|GetSprite) (Math|Rotator|MakeRotator 0.0 0.0 (+ (.Yaw (Math|Rotator|BreakRotator (Math|Rotator|FindLookatRotation (Variables|/Game/PlayerControllers/Chef/Blueprints/BP_ThirdPersonCharacter.BP_ThirdPersonCharacter_C|GetCamPosition _output_get) (Transformation|GetWorldLocation (Variables|/Script/Engine.Character|GetCapsuleComponent _returnvalue))))) -9e+01)) false false))

(fn ConstructionScript)

(fn GetSprite
  (switch Utilities|FlowControl|Switch|SwitchonEnum_CookingIngredients (Variables|Default|GetIngredientType)
    (:NewEnumerator0
      (return "/Game/Sprites/cheese_testsprite_Sprite.cheese_testsprite_Sprite"))
    (:NewEnumerator1
      (return "/Game/Sprites/buns_testsprite_Sprite.buns_testsprite_Sprite"))
    (:NewEnumerator2
      (return "/Game/Sprites/steak_testsprite_Sprite.steak_testsprite_Sprite"))))

(fn UpdateFoodSprite
  (params (FoodType :type Enum_CookingIngredients%20Enum :default "NewEnumerator0"))
  (Variables|Default|SetIngredientType FoodType)
  (bind _newparam (CallFunction|GetSprite))
  (Rendering|Components|Sprite|SetSprite (Variables|Default|GetSprite) _newparam))