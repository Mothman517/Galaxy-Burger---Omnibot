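; BP_FoodContainer is a world container for one food type (cheese, buns or beef), shown as a Paper2D sprite.
; On BeginPlay it yaws the sprite once toward the player's camera position and sets its image from FoodType via UpdateSprite.
; Box overlaps with Player-tagged actors set or clear NearFoodContainer and CurrentContainer on the cached player character.
; TakeFood is an empty stub.
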(event OnComponentBeginOverlap(Box)
  (params (OverlappedComponent :type Primitive%20Component%20Object%20Reference) (OtherActor :type Actor%20Object%20Reference) (OtherComp :type Primitive%20Component%20Object%20Reference) (OtherBodyIndex :type Integer) (bFromSweep :type Boolean) (SweepResult :type Hit%20Result%20Structure%20%28by%20ref%29))
  (bind _playerref (Variables|Default|GetPlayerRef))
  ;[0.15 0.15 0.15 0.5] Toggle Collision
  (if (Actor|ActorHasTag OtherActor "Player")
    (Development|PrintString "IN")
    (Variables|/Game/PlayerControllers/Chef/Blueprints/BP_ThirdPersonCharacter.BP_ThirdPersonCharacter_C|SetnearFoodContainer _playerref true)
    (Variables|/Game/PlayerControllers/Chef/Blueprints/BP_ThirdPersonCharacter.BP_ThirdPersonCharacter_C|SetcurrentContainer _playerref self)))

(event OnComponentEndOverlap(Box)
  (params (OverlappedComponent :type Primitive%20Component%20Object%20Reference) (OtherActor :type Actor%20Object%20Reference) (OtherComp :type Primitive%20Component%20Object%20Reference) (OtherBodyIndex :type Integer))
  (bind _playerref (Variables|Default|GetPlayerRef))
  ;[0.15 0.15 0.15 0.5] Toggle Collision
  (if (Actor|ActorHasTag OtherActor "Player")
    (Development|PrintString "OUT")
    (Variables|/Game/PlayerControllers/Chef/Blueprints/BP_ThirdPersonCharacter.BP_ThirdPersonCharacter_C|SetnearFoodContainer _playerref false)
    (Variables|/Game/PlayerControllers/Chef/Blueprints/BP_ThirdPersonCharacter.BP_ThirdPersonCharacter_C|SetcurrentContainer _playerref 0)))

(event EventBeginPlay
  ;[0.15 0.15 0.15 0.5] StartUp
  (bind _asbp_third_person_character (Utilities|Casting|CastToBP_ThirdPersonCharacter (Game|GetPlayerCharacter 0)))
  (bind _output_get (Variables|Default|SetPlayerRef _asbp_third_person_character))
  (Transformation|SetWorldRotation (Variables|Default|GetPaperSprite) (Math|Rotator|MakeRotator 0.0 0.0 (+ (.Yaw (Math|Rotator|BreakRotator (Math|Rotator|FindLookatRotation (Variables|/Game/PlayerControllers/Chef/Blueprints/BP_ThirdPersonCharacter.BP_ThirdPersonCharacter_C|GetCamPosition _output_get) (Transformation|GetWorldLocation (Variables|Default|GetPaperSprite))))) -9e+01)) false false)
  (bind _newparam (CallFunction|UpdateSprite (Variables|Default|GetFoodType)))
  (Rendering|Components|Sprite|SetSprite (Variables|Default|GetPaperSprite) _newparam))

(fn ConstructionScript)

(fn UpdateSprite
  (params (Ingredient :type Enum_CookingIngredients%20Enum :default "NewEnumerator0"))
  (switch Utilities|FlowControl|Switch|SwitchonEnum_CookingIngredients Ingredient
    (:NewEnumerator0
      (return "/Game/Sprites/cheese_testsprite_Sprite.cheese_testsprite_Sprite"))
    (:NewEnumerator1
      (return "/Game/Sprites/buns_testsprite_Sprite.buns_testsprite_Sprite"))
    (:NewEnumerator2
      (return "/Game/Sprites/steak_testsprite_Sprite.steak_testsprite_Sprite"))))

(fn TakeFood)