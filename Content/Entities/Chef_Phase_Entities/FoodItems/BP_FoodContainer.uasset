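; BP_FoodContainer is an ingredient container for the chef phase, marked by a billboard sprite of the food it holds.
; On BeginPlay it caches the BP_PlayerChef reference and uses UpdateSprite to map its FoodType to that sprite.
; Its box overlap events set the chef's NearFoodContainer flag and CurrentContainer reference when the player enters, and clear both on exit, with debug prints.
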(event OnComponentBeginOverlap(Box)
  (params (OverlappedComponent :type Primitive%20Component%20Object%20Reference) (OtherActor :type Actor%20Object%20Reference) (OtherComp :type Primitive%20Component%20Object%20Reference) (OtherBodyIndex :type Integer) (bFromSweep :type Boolean) (SweepResult :type Hit%20Result%20Structure%20%28by%20ref%29))
  (bind _playerref (Variables|Default|GetPlayerRef))
  ;[0.15 0.15 0.15 0.5] Toggle Collision
  (if (Actor|ActorHasTag OtherActor "Player")
    (Development|PrintString "IN")
    (Variables|/Game/PlayerControllers/Chef/Blueprints/BP_PlayerChef.BP_PlayerChef_C|SetNear%20Food%20Container _playerref true)
    (Variables|/Game/PlayerControllers/Chef/Blueprints/BP_PlayerChef.BP_PlayerChef_C|SetcurrentContainer _playerref self)))

(event OnComponentEndOverlap(Box)
  (params (OverlappedComponent :type Primitive%20Component%20Object%20Reference) (OtherActor :type Actor%20Object%20Reference) (OtherComp :type Primitive%20Component%20Object%20Reference) (OtherBodyIndex :type Integer))
  (bind _playerref (Variables|Default|GetPlayerRef))
  ;[0.15 0.15 0.15 0.5] Toggle Collision
  (if (Actor|ActorHasTag OtherActor "Player")
    (Development|PrintString "OUT")
    (Variables|/Game/PlayerControllers/Chef/Blueprints/BP_PlayerChef.BP_PlayerChef_C|SetNear%20Food%20Container _playerref false)
    (Variables|/Game/PlayerControllers/Chef/Blueprints/BP_PlayerChef.BP_PlayerChef_C|SetcurrentContainer _playerref 0)))

(event EventBeginPlay
  ;[0.15 0.15 0.15 0.5] StartUp
  (bind _asbp_player_chef (Utilities|Casting|CastToBP_PlayerChef (Game|GetPlayerCharacter 0)))
  (Variables|Default|SetPlayerRef _asbp_player_chef)
  (bind _texture (CallFunction|UpdateSprite (Variables|Default|GetFoodType)))
  (Rendering|Components|Sprite|SetSprite (Variables|Default|GetBillboard) _texture))

(fn ConstructionScript)

(fn UpdateSprite
  (params (Ingredient :type Enum_CookingIngredients%20Enum :default "NewEnumerator0"))
  (switch Utilities|FlowControl|Switch|SwitchonEnum_CookingIngredients Ingredient
    (:NewEnumerator0
      (return "/Game/Textures/Sprites/New_Food_Sprites/UI_IngredientCheese.UI_IngredientCheese"))
    (:NewEnumerator1
      (return "/Game/Textures/Sprites/New_Food_Sprites/UI_IngredientBun.UI_IngredientBun"))
    (:NewEnumerator2
      (return "/Game/Textures/Sprites/New_Food_Sprites/UI_IngredientCookedPatty.UI_IngredientCookedPatty"))
    (:NewEnumerator3
      (return "/Game/Textures/Sprites/New_Food_Sprites/UI_IngredientLettuce.UI_IngredientLettuce"))
    (:NewEnumerator5
      (return "/Game/Textures/Sprites/New_Food_Sprites/UI_IngredientTomato.UI_IngredientTomato"))
    (:NewEnumerator17
      (return "/Game/Textures/Sprites/sliced_Tomato_testsprite.sliced_Tomato_testsprite"))
    (:NewEnumerator6
      (return "/Game/Textures/Sprites/New_Food_Sprites/UI_IngredientPotato.UI_IngredientPotato"))
    (:NewEnumerator18
      (return "/Game/Textures/Sprites/New_Food_Sprites/UI_IngredientRawFries.UI_IngredientRawFries"))
    (:NewEnumerator7
      (return "/Game/Textures/Sprites/New_Food_Sprites/UI_IngredientChicken.UI_IngredientChicken"))
    (:NewEnumerator14
      (return "/Game/Textures/Sprites/New_Food_Sprites/UI_IngredientCutChicken.UI_IngredientCutChicken"))))