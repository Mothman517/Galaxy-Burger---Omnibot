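; Base pickup for chef-phase food, displayed as either a raw ingredient sprite or a 3D meal.
; Ingredients pick a billboard sprite by IngredientType, while meals spawn burger, fries or nugget meshes at runtime under DisplaySpawnPoint, which spins on Tick.
; Burgers stack AddedIngredients between buns at rising heights with random yaw.
; Sphere overlap with the player sets or clears this actor as the chef's ClosestPickup.
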(event OnComponentBeginOverlap(Sphere1)
  (params (OverlappedComponent :type Primitive%20Component%20Object%20Reference) (OtherActor :type Actor%20Object%20Reference) (OtherComp :type Primitive%20Component%20Object%20Reference) (OtherBodyIndex :type Integer) (bFromSweep :type Boolean) (SweepResult :type Hit%20Result%20Structure%20%28by%20ref%29))
  ;[0.15 0.15 0.15 0.5] Collision Detection Toggles
  (if (Actor|ActorHasTag OtherActor "Player")
    (Variables|Default|SetisOverlapping true)
    (Variables|/Game/PlayerControllers/Chef/Blueprints/BP_PlayerChef.BP_PlayerChef_C|SetclosestPickup (Variables|Default|GetPlayerRef) self)))

(event OnComponentEndOverlap(Sphere1)
  (params (OverlappedComponent :type Primitive%20Component%20Object%20Reference) (OtherActor :type Actor%20Object%20Reference) (OtherComp :type Primitive%20Component%20Object%20Reference) (OtherBodyIndex :type Integer))
  ;[0.15 0.15 0.15 0.5] Collision Detection Toggles
  (if (Actor|ActorHasTag OtherActor "Player")
    (Variables|Default|SetisOverlapping false)
    (Variables|/Game/PlayerControllers/Chef/Blueprints/BP_PlayerChef.BP_PlayerChef_C|SetclosestPickup (Variables|Default|GetPlayerRef) 0)))

(event Custom|Set%20Visuals
  ;[0.15 0.15 0.15 0.5] Set Visuals
  (if (Variables|Default|GetIs%20A%20Meal)
    (CallFunction|ChooseMesh)
    (else
      (bind _texture (CallFunction|GetSprite))
      (Rendering|Components|Sprite|SetSprite (Variables|Default|GetBillboard) _texture))))

(event EventBeginPlay
  ;[0.15 0.15 0.15 0.5] Setting the sprite + Billboarding
  (bind _asbp_player_chef (Utilities|Casting|CastToBP_PlayerChef (Game|GetPlayerCharacter 0)))
  (Variables|Default|SetPlayerRef _asbp_player_chef)
  (CallFunction|SetVisuals))

(event EventTick
  (params (DeltaSeconds :type Float%20%28single-precision%29))
  (bind _displayspawnpoint (Variables|Default|GetDisplaySpawnPoint))
  ;[0.15 0.15 0.15 0.5] Spin Meshes
  (if (Variables|Default|GetIs%20A%20Meal)
    (Transformation|SetWorldRotation _displayspawnpoint (Math|Rotator|MakeRotator 0.0 0.0 (+ (* DeltaSeconds (Variables|Default|GetRotationSpeed)) (.yaw (Transformation|GetWorldRotation _displayspawnpoint)))) false false)))

(event Custom|Build%20Burger
  ;[0.15 0.15 0.15 0.5] Burger
  ;;[0.15 0.15 0.15 0.5] Add Bottom Bun
  (Variables|Default|SetHeight 2.0)
  (bind _returnvalue (AddComponent|AddStaticMeshComponent false))
  (Transformation|AttachComponentToComponent _returnvalue (Variables|Default|GetDisplaySpawnPoint) "None" "KeepRelative" "KeepRelative" "KeepRelative" true)
  (Collision|SetCollisionEnabled _returnvalue "NoCollision")
  (Components|StaticMesh|SetStaticMesh _returnvalue "/Game/Models/bottom_bun.bottom_bun")
  ;;[0.15 0.15 0.15 0.5] Add Inner Ingredients
  (for _array_element (Variables|Default|GetAdded%20Ingredients)
    (bind _returnvalue_2 (AddComponent|AddStaticMeshComponent false))
    (Transformation|AttachComponentToComponent _returnvalue_2 (Variables|Default|GetDisplaySpawnPoint) "None" "KeepRelative" "KeepRelative" "KeepRelative" true)
    (Collision|SetCollisionEnabled _returnvalue_2 "NoCollision")
    (bind _mesh (CallFunction|GetStaticMesh _array_element))
    (Components|StaticMesh|SetStaticMesh _returnvalue_2 _mesh)
    (Transformation|SetRelativeLocation _returnvalue_2 (Math|Vector|MakeVector 0.0 0.0 (Variables|Default|GetHeight)) false false)
    (Variables|Default|SetHeight (+ (Variables|Default|GetHeight) 2.0))
    (Transformation|SetWorldRotation _returnvalue_2 (Math|Rotator|MakeRotator 0.0 0.0 (Math|Random|RandomFloatinRange 0.0 3.6e+02)) false false))
  ;;[0.15 0.15 0.15 0.5] Add Top Bun
  (bind _returnvalue_3 (AddComponent|AddStaticMeshComponent false))
  (Transformation|AttachComponentToComponent _returnvalue_3 (Variables|Default|GetDisplaySpawnPoint) "None" "KeepRelative" "KeepRelative" "KeepRelative" true)
  (Collision|SetCollisionEnabled _returnvalue_3 "NoCollision")
  (Components|StaticMesh|SetStaticMesh _returnvalue_3 "/Game/Models/top_bun.top_bun")
  (Transformation|SetRelativeLocation _returnvalue_3 (Math|Vector|MakeVector 0.0 0.0 (Variables|Default|GetHeight)) false false))

(event Custom|Clear%20Meshes
  (bind _displayspawnpoint (Variables|Default|GetDisplaySpawnPoint))
  (bind _children (Components|GetChildrenComponents _displayspawnpoint false))
  ;[0.15 0.15 0.15 0.5] Clear Meshes
  (bind _arrayelement (Utilities|Array|ReverseforEachLoop _children)
    (:LoopBody
      (Components|DestroyComponent _arrayelement))
    (:Completed
      (Utilities|Array|Resize _children 0))))

(event Custom|Build%20Fries
  ;[0.15 0.15 0.15 0.5] Fries
  (Variables|Default|SetHeight 2.0)
  (bind _returnvalue (AddComponent|AddStaticMeshComponent false))
  (Transformation|AttachComponentToComponent _returnvalue (Variables|Default|GetDisplaySpawnPoint) "None" "KeepRelative" "KeepRelative" "KeepWorld" true)
  (Collision|SetCollisionEnabled _returnvalue "NoCollision")
  (Components|StaticMesh|SetStaticMesh _returnvalue "/Game/Models/Fries_READY.Fries_READY"))

(event Custom|Build%20Nugget
  ;[0.15 0.15 0.15 0.5] Build Nugget
  (Variables|Default|SetHeight 2.0)
  (bind _returnvalue (AddComponent|AddStaticMeshComponent false))
  (Transformation|AttachComponentToComponent _returnvalue (Variables|Default|GetDisplaySpawnPoint) "None" "KeepRelative" "KeepRelative" "KeepWorld" true)
  (Collision|SetCollisionEnabled _returnvalue "NoCollision")
  (Components|StaticMesh|SetStaticMesh _returnvalue "/Game/Models/NuggetFried.NuggetFried"))

(fn ConstructionScript)

(fn GetSprite
  (switch Utilities|FlowControl|Switch|SwitchonEnum_CookingIngredients (Variables|Default|GetIngredientType)
    (:NewEnumerator0
      (return "/Game/Textures/Sprites/New_Food_Sprites/UI_IngredientCheese.UI_IngredientCheese"))
    (:NewEnumerator1
      (return "/Game/Textures/Sprites/New_Food_Sprites/UI_IngredientBun.UI_IngredientBun"))
    (:NewEnumerator2
      (return "/Game/Textures/Sprites/New_Food_Sprites/UI_IngredientCookedPatty.UI_IngredientCookedPatty"))
    (:NewEnumerator3
      (return "/Game/Textures/Sprites/New_Food_Sprites/UI_IngredientLettuce.UI_IngredientLettuce"))
    (:NewEnumerator5
      (return "/Game/Textures/Sprites/New_Food_Sprites/UI_IngredientTomato.UI_IngredientTomato"))
    (:NewEnumerator17
      (return "/Game/Textures/Sprites/New_Food_Sprites/TEMP_UI_IngredientSlicedTomato.TEMP_UI_IngredientSlicedTomato"))
    (:NewEnumerator6
      (return "/Game/Textures/Sprites/New_Food_Sprites/UI_IngredientPotato.UI_IngredientPotato"))
    (:NewEnumerator18
      (return "/Game/Textures/Sprites/New_Food_Sprites/UI_IngredientRawFries.UI_IngredientRawFries"))
    (:NewEnumerator7
      (return "/Game/Textures/Sprites/New_Food_Sprites/UI_IngredientChicken.UI_IngredientChicken"))
    (:NewEnumerator12
      (return 0))
    (:NewEnumerator14
      (return "/Game/Textures/Sprites/New_Food_Sprites/UI_IngredientCutChicken.UI_IngredientCutChicken"))))

(fn UpdateFoodSprite
  (params (FoodType :type Enum_CookingIngredients%20Enum :default "NewEnumerator0"))
  (Variables|Default|SetIngredientType FoodType)
  (bind _texture (CallFunction|GetSprite))
  (Rendering|Components|Sprite|SetSprite (Variables|Default|GetBillboard) _texture))

(fn ChooseMesh
  (switch Utilities|FlowControl|Switch|SwitchonEnum_CookingIngredients (Variables|Default|GetIngredientType)
    (:NewEnumerator12
      (CallFunction|BuildBurger))
    (:NewEnumerator13
      (CallFunction|BuildFries))
    (:NewEnumerator19
      (CallFunction|BuildNugget))))

(fn GetStaticMesh
  (params (Ingredient :type Enum_CookingIngredients%20Enum :default "NewEnumerator0"))
  (switch Utilities|FlowControl|Switch|SwitchonEnum_CookingIngredients Ingredient
    (:NewEnumerator0
      (return "/Game/Models/cheese.cheese"))
    (:NewEnumerator1
      (return "/Game/Models/bottom_bun.bottom_bun"))
    (:NewEnumerator2
      (return "/Game/Models/patty.patty"))
    (:NewEnumerator3
      (return "/Game/Models/lettuce.lettuce"))
    (:NewEnumerator5
      (return "/Game/Models/tomatoes.tomatoes"))))