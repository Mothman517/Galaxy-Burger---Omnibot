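; BP_OrderManager spawns customer orders during the chef phase, scaling their contents with the current game day.
; On a Tick timer, it rolls against a failure counter, so spawn odds rise after each miss.
; Orders hold a random burger, whose length and ingredient pool depend on the day, plus sides unlocked on later days.
; SummonCustomer assigns each order to the first inactive BP_Order found at BeginPlay; debug key 8 forces one.
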(event EventBeginPlay
  (bind _asbp_player_chef (Utilities|Casting|CastToBP_PlayerChef (Game|GetPlayerCharacter 0)))
  (Variables|Default|SetPlayerRef _asbp_player_chef)
  (bind _outactors (Actor|GetAllActorsOfClass "/Game/Entities/Chef_Phase_Entities/Stationary/BP_Order.BP_Order_C"))
  (Variables|Default|SetOrder%20List _outactors)
  (bind _asbp_game_data (Utilities|Casting|CastToBP_GameData (Game|GetGameInstance)))
  (bind _output_get (Variables|Default|SetGameData%20Ref _asbp_game_data))
  (Development|PrintString (Utilities|String|ToString(Integer) (Variables|/Game/Game_Data/BP_GameData.BP_GameData_C|GetDay _output_get))))

(event Collision|EventActorBeginOverlap
  (params (OtherActor :type Actor%20Object%20Reference)))

(event EventTick
  (params (DeltaSeconds :type Float%20%28single-precision%29))
  (Variables|Default|SetTimer (+ (Variables|Default|GetTimer) DeltaSeconds))
  (if (>= (+ (Variables|Default|GetTimer) DeltaSeconds) (Variables|Default|GetTime%20To%20Spawn))
    (if (< (Math|Random|RandomIntegerinRange 0 21) (Variables|Default|GetCustomer%20Spawn%20Tick))
      (Variables|Default|SetCustomer%20Spawn%20Tick 0)
      (bind _order (CallFunction|CreateOrder))
      (CallFunction|SummonCustomer _order)
      (else
        (Variables|Default|SetCustomer%20Spawn%20Tick (+ (Variables|Default|GetCustomer%20Spawn%20Tick) 1))))
    (Variables|Default|SetTimer 0.0)))

(event Input|KeyboardEvents|DebugKey8
  (params (Key :type Key%20Structure) (ActionValue :type Input%20Action%20Value%20Structure))
  (:Pressed
    (bind _burger (CallFunction|GenerateBurger 2))
    (CallFunction|SummonCustomer (Utilities|Array|MakeArray _burger))))

(fn ConstructionScript)

(fn CreateOrder
  (bind _gamedata_ref (Variables|Default|GetGameData%20Ref))
  (bind _day (Variables|/Game/Game_Data/BP_GameData.BP_GameData_C|GetDay _gamedata_ref))
  ;[0.15 0.15 0.15 0.5] Add Burger
  (Development|PrintString (Utilities|String|ToString(Integer) _day))
  (bind _burger (CallFunction|GenerateBurger (Math|Random|RandomIntegerinRange 1 (+ _day 1))))
  (Utilities|Array|Add (LocalVariables|Getnew%20Order) _burger)
  ;[0.15 0.15 0.15 0.5] Can order fries?
  (if (> (Variables|/Game/Game_Data/BP_GameData.BP_GameData_C|GetDay (Variables|Default|GetGameData%20Ref)) 1)
    ;[0.15 0.15 0.15 0.5] Add Fries
    (Utilities|Array|Add (LocalVariables|Getnew%20Order) (Utilities|Struct|MakeST_Ingredient "NewEnumerator13" "NewEnumerator20" true))
    ;[0.15 0.15 0.15 0.5] Can order nuggets?
    (if (> (Variables|/Game/Game_Data/BP_GameData.BP_GameData_C|GetDay (Variables|Default|GetGameData%20Ref)) 2)
      ;[0.15 0.15 0.15 0.5] Add Nuggets
      (Utilities|Array|Add (LocalVariables|Getnew%20Order) (Utilities|Struct|MakeST_Ingredient "NewEnumerator19" "NewEnumerator20" true))
      ;[0.15 0.15 0.15 0.5] Can order nuggets?
      (if (> (Variables|/Game/Game_Data/BP_GameData.BP_GameData_C|GetDay (Variables|Default|GetGameData%20Ref)) 3)
        ;[0.15 0.15 0.15 0.5] Add Nuggets
        (Utilities|Array|Add (LocalVariables|Getnew%20Order) (Utilities|Struct|MakeST_Ingredient "NewEnumerator15" "NewEnumerator20" true)))))
  (return (LocalVariables|Getnew%20Order)))

(fn GenerateBurger
  (params (Length :type Integer))
  (bind _elligle_ingredients_uno (LocalVariables|GetElligle%20Ingredients%20UNO))
  (bind _elligle_ingredients_dos (LocalVariables|GetElligle%20Ingredients%20DOS))
  (bind _created_order (LocalVariables|GetCreated%20Order))
  (Development|PrintString "YES")
  (while (> Length (LocalVariables|Getindex))
    (if (>= (Variables|/Game/Game_Data/BP_GameData.BP_GameData_C|GetDay (Variables|Default|GetGameData%20Ref)) 3)
      (Utilities|Array|Add _created_order (Utilities|Array|Get(acopy) _elligle_ingredients_dos (- (Math|Random|RandomIntegerinRange 1 (Utilities|Array|Length _elligle_ingredients_dos)) 1)))
      (else
        (Utilities|Array|Add _created_order (Utilities|Array|Get(acopy) _elligle_ingredients_uno (- (Math|Random|RandomIntegerinRange 1 (Utilities|Array|Length _elligle_ingredients_uno)) 1)))))
    (LocalVariables|Setindex (+ (LocalVariables|Getindex) 1)))
  (return (Utilities|Struct|MakeST_Ingredient "NewEnumerator12" _created_order true)))

(fn SummonCustomer
  (params (Order :type Array%20of%20ST%20Ingredient%20Structures))
  (bind (_array_element _array_index) (Utilities|Array|ForEachLoopwithBreak (Variables|Default|GetOrder%20List) :!label _label)
    (:LoopBody
      (if (not (Variables|/Game/Entities/Chef_Phase_Entities/Stationary/BP_Order.BP_Order_C|GetIs%20Active _array_element))
        (LocalVariables|SetPindex _array_index)
        (LocalVariables|SetTarget%20Order _array_element)
        (Development|PrintString "customer")
        (goto _label Break)))
    (:Completed
      (if (!= (LocalVariables|GetPindex) -1)
        (Default|SetOrder (LocalVariables|GetTarget%20Order) Order)
        (else
          (Development|PrintString "NO EMPTY SLOTS"))))))