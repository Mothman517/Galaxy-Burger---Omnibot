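; Chef-phase combo station that assembles a meal from a base food plus eligible ingredients, currently with visuals only for burgers.
; AddIngredient requires InputFood to start, immediately marking the meal done, then records eligible additions.
; Each accepted item passes through ChooseMesh to MakeBurger, which stacks a runtime static mesh at increasing height with random yaw.
; GetOutput returns OutputFood with its additions; ResetBoard clears meal state after calling the parent.
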(event EventBeginPlay
  (|CallParentFunction) ; This node is disabled and will not be called.\nDrag off pins to build functionality.
)

(event Collision|EventActorBeginOverlap
  (params (OtherActor :type Actor%20Object%20Reference)))

(event EventTick
  (params (DeltaSeconds :type Float%20%28single-precision%29)))

(event Custom|Make%20Burger
  (params (Ingredient :type Enum_CookingIngredients%20Enum :default "NewEnumerator0"))
  (bind _returnvalue (AddComponent|AddStaticMeshComponent false))
  (Transformation|AttachComponentToComponent _returnvalue (Variables|Default|GetIngredient%20Spawn%20Point) "None" "KeepRelative" "KeepRelative" "KeepRelative" true)
  (bind _mesh (CallFunction|GetMesh Ingredient))
  (Components|StaticMesh|SetStaticMesh _returnvalue _mesh)
  (Transformation|SetRelativeLocation _returnvalue (Math|Vector|MakeVector 0.0 0.0 (Variables|Default|GetHeight)) false false)
  (Variables|Default|SetHeight (+ (Variables|Default|GetHeight) 2.0))
  (Transformation|SetWorldRotation _returnvalue (Math|Rotator|MakeRotator 0.0 0.0 (Math|Random|RandomFloatinRange 0.0 3.6e+02)) false false))

(fn ConstructionScript
  (|CallParentFunction))

(fn ResetBoard
  (|CallParentFunction)
  (Utilities|Array|Clear (Variables|Default|GetAdded%20Ingredients))
  (Variables|Default|SetHeight 0.0)
  (Variables|Default|SetMeal%20In%20Progress false)
  (Variables|Default|SetIs%20Done false)
  (Development|PrintString "67!!!"))

(fn GetOutput
  (return (Utilities|Struct|MakeST_Ingredient (Variables|Default|GetOutput%20Food) (Variables|Default|GetAdded%20Ingredients) true) (Variables|Default|GetMeal%20In%20Progress)))

(fn ChooseMesh
  (params (Ingredient%20To%20Add :type Enum_CookingIngredients%20Enum :default "NewEnumerator0"))
  (switch Utilities|FlowControl|Switch|SwitchonEnum_CookingIngredients (Variables|Default|GetOutput%20Food)
    (:NewEnumerator12
      (CallFunction|MakeBurger Ingredient%20To%20Add))))

(fn AddIngredient
  (params (Input :type Enum_CookingIngredients%20Enum :default "NewEnumerator0"))
  (if (Variables|Default|GetMeal%20In%20Progress)
    ;[0.15 0.15 0.15 0.5] Add Ingredients
    (if (Utilities|Array|ContainsItem (Variables|Default|GetElgible%20Ingredients) Input)
      (Development|PrintString "Adding Ingredient")
      (Utilities|Array|Add (Variables|Default|GetAdded%20Ingredients) Input)
      (CallFunction|ChooseMesh Input)
      (return true)
      (else
        (Development|PrintString "NOT ADDING")
        (return false)))
    (else
      ;[0.15 0.15 0.15 0.5] Start Building A Meal
      (if (Utilities|Enum|Equal(Enum) Input (Variables|Default|GetInput%20Food))
        (Development|PrintString "Started Building")
        (bind _output_get (Variables|Default|SetMeal%20In%20Progress true))
        (Variables|Default|SetIs%20Done _output_get)
        (CallFunction|ChooseMesh Input)
        (return true)
        (else
          (Development|PrintString "NOT BUILDING")
          (return false))))))