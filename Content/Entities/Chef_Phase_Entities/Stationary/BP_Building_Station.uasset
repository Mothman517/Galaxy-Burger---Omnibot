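; Building station for the chef phase, where ingredients are assembled into a meal, currently with burger visuals only.
; The base input food starts a meal, after which only eligible ingredients are accepted and recorded.
; Accepted items spawn static mesh components at a spawn point, stacked upward with random yaw, and ResetBoard clears them.
; Box overlaps toggle the player's NearStation flag but set CurrentStation to None.
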(event OnComponentBeginOverlap(Box)
  (params (OverlappedComponent :type Primitive%20Component%20Object%20Reference) (OtherActor :type Actor%20Object%20Reference) (OtherComp :type Primitive%20Component%20Object%20Reference) (OtherBodyIndex :type Integer) (bFromSweep :type Boolean) (SweepResult :type Hit%20Result%20Structure%20%28by%20ref%29))
  (bind _playerref (Variables|Default|GetPlayerRef))
  ;[0.15 0.15 0.15 0.5] Is Player close to a station
  (if (Actor|ActorHasTag OtherActor "Player")
    (Variables|/Game/PlayerControllers/Chef/Blueprints/BP_PlayerChef.BP_PlayerChef_C|SetNear%20Station _playerref true)
    (Variables|/Game/PlayerControllers/Chef/Blueprints/BP_PlayerChef.BP_PlayerChef_C|Setcurrent%20Station _playerref 0)))

(event OnComponentEndOverlap(Box)
  (params (OverlappedComponent :type Primitive%20Component%20Object%20Reference) (OtherActor :type Actor%20Object%20Reference) (OtherComp :type Primitive%20Component%20Object%20Reference) (OtherBodyIndex :type Integer))
  (bind _playerref (Variables|Default|GetPlayerRef))
  ;[0.15 0.15 0.15 0.5] Is Player close to a station
  (if (Actor|ActorHasTag OtherActor "Player")
    (Variables|/Game/PlayerControllers/Chef/Blueprints/BP_PlayerChef.BP_PlayerChef_C|SetNear%20Station _playerref false)
    (Variables|/Game/PlayerControllers/Chef/Blueprints/BP_PlayerChef.BP_PlayerChef_C|Setcurrent%20Station _playerref 0)))

(event EventBeginPlay
  (bind _asbp_player_chef (Utilities|Casting|CastToBP_PlayerChef (Game|GetPlayerCharacter 0)))
  (Variables|Default|SetPlayerRef _asbp_player_chef))

(event Custom|Make%20Burger
  (params (Ingredient :type Enum_CookingIngredients%20Enum :default "NewEnumerator0"))
  (bind _returnvalue (AddComponent|AddStaticMeshComponent false))
  (Transformation|AttachComponentToComponent _returnvalue (Variables|Default|GetIngredient%20Spawn%20Point) "None" "KeepRelative" "KeepRelative" "KeepRelative" true)
  (CallFunction|GetMesh Ingredient)
  (Components|StaticMesh|SetStaticMesh _returnvalue "/Game/Models/top_bun.top_bun")
  (Transformation|SetRelativeLocation _returnvalue (Math|Vector|MakeVector 0.0 0.0 (Variables|Default|GetHeight)) false false)
  (Variables|Default|SetHeight (+ (Variables|Default|GetHeight) 2.0))
  (Transformation|SetWorldRotation _returnvalue (Math|Rotator|MakeRotator 0.0 0.0 (Math|Random|RandomFloatinRange 0.0 3.6e+02)) false false))

(fn ConstructionScript)

(fn AddIngredient
  (params (Input :type Enum_CookingIngredients%20Enum :default "NewEnumerator0"))
  (if (Variables|Default|GetMeal%20In%20Progress)
    ;[0.15 0.15 0.15 0.5] Add Ingredients
    (if (Utilities|Array|ContainsItem (Variables|Default|GetElgible%20Ingredients) Input)
      (Development|PrintString "Adding Ingredient")
      (Utilities|Array|Add (Variables|Default|GetAdded%20Ingredients) Input)
      (CallFunction|ChooseMesh Input)
      (return true)
      (else
        (Development|PrintString "NOT ADDING")
        (return false)))
    (else
      ;[0.15 0.15 0.15 0.5] Start Building A Meal
      (if (Utilities|Enum|Equal(Enum) Input (Variables|Default|GetInput%20Food))
        (Development|PrintString "Started Building")
        (Variables|Default|SetMeal%20In%20Progress true)
        (CallFunction|ChooseMesh Input)
        (return true)
        (else
          (Development|PrintString "NOT BUILDING")
          (return false))))))

(fn ChooseMesh
  (params (Ingredient%20To%20Add :type Enum_CookingIngredients%20Enum :default "NewEnumerator0"))
  (switch Utilities|FlowControl|Switch|SwitchonEnum_CookingIngredients (Variables|Default|GetOutput%20Food)
    (:NewEnumerator12
      (CallFunction|MakeBurger Ingredient%20To%20Add))))

(fn GetMesh
  (params (Ingredient :type Enum_CookingIngredients%20Enum :default "NewEnumerator0"))
  (switch Utilities|FlowControl|Switch|SwitchonEnum_CookingIngredients Ingredient
    (:NewEnumerator0
      (return "/Game/Models/cheese.cheese"))
    (:NewEnumerator1
      (return "/Game/Models/bottom_bun.bottom_bun"))
    (:NewEnumerator2
      (return "/Game/Models/patty.patty"))
    (:NewEnumerator3
      (return "/Game/Models/lettuce.lettuce"))
    (:NewEnumerator5
      (return "/Game/Models/tomatoes.tomatoes"))))

(fn ResetBoard
  (bind _arrayelement (Utilities|Array|ReverseforEachLoop (Components|GetChildrenComponents (Variables|Default|GetIngredient%20Spawn%20Point) false))
    (:LoopBody
      (Components|DestroyComponent _arrayelement))
    (:Completed
      (Utilities|Array|Clear (Variables|Default|GetAdded%20Ingredients))
      (Variables|Default|SetMeal%20In%20Progress true)
      (Variables|Default|SetHeight 0.0))))