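; Kitchen machine station, apparently for ice cream, that prepares a meal over time and can break down.
; Tick drives one timer for preparing or hold-to-repair (releasing Interact restarts repair), feeding a progress widget turned toward the player camera at BeginPlay.
; GetOutput yields the meal once done.
; ResetBoard clears the station, raising break chance and rolling for breakage after normal use, or zeroing that chance after repair.
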(event EventBeginPlay
  (bind _playerref (Variables|Default|GetPlayerRef))
  (bind _widget (Variables|Default|GetWidget))
  (bind _returnvalue (Transformation|GetWorldLocation _widget))
  (bind _camposition (Variables|/Game/PlayerControllers/Chef/Blueprints/BP_PlayerChef.BP_PlayerChef_C|GetCamPosition _playerref))
  (bind _returnvalue_2 (Math|Rotator|FindLookatRotation _returnvalue _camposition))
  (|CallParentFunction)
  (Transformation|SetWorldRotation _widget (Math|Rotator|MakeRotator 0.0 (.pitch _returnvalue_2) (.yaw _returnvalue_2)) false false)
  (bind _asprogress_bar_ui (Utilities|Casting|CastToProgress_Bar_UI (UserInterface|GetWidget (Variables|Default|GetWidget))))
  (Variables|Default|SetUI%20Reference _asprogress_bar_ui))

(event Collision|EventActorBeginOverlap
  (params (OtherActor :type Actor%20Object%20Reference)))

(event EventTick
  (params (DeltaSeconds :type Float%20%28single-precision%29))
  (if (Variables|Default|GetMeal%20In%20Progress)
    (if (Variables|Default|GetIsBroken)
      (if (Variables|/Game/PlayerControllers/Chef/Blueprints/BP_PlayerChef.BP_PlayerChef_C|GetHolding%20Interact (Variables|Default|GetPlayerRef))
        (bind _output_get (Variables|Default|SetTimer (+ DeltaSeconds (Variables|Default|GetTimer))))
        (else
          (Variables|Default|SetTimer 0.0)))
      (if (>= _output_get (Variables|Default|GetTime%20To%20Repair))
        (CallFunction|ResetBoard))
      (Default|SetPercent (Variables|Default|GetUI%20Reference) (/ (Variables|Default|GetTimer) (Variables|Default|GetTime%20To%20Repair)))
      (else
        ;[0.15 0.15 0.15 0.5] Preparing
        (bind _output_get_2 (Variables|Default|SetTimer (+ DeltaSeconds (Variables|Default|GetTimer))))
        (if (>= _output_get_2 (Variables|Default|GetTime%20To%20Prepare))
          (Variables|Default|SetIs%20Done true))
        (Default|SetPercent (Variables|Default|GetUI%20Reference) (/ (Variables|Default|GetTimer) (Variables|Default|GetTime%20To%20Prepare)))))))

(fn ConstructionScript
  (|CallParentFunction))

(fn MakeCream
  (bind _ui_reference (Variables|Default|GetUI%20Reference))
  (Variables|Default|SetMeal%20In%20Progress true)
  (Development|PrintString "creaming")
  (Default|ToggleVisibility _ui_reference true)
  (Default|SetImage _ui_reference (Variables|Default|GetOutput%20Food)))

(fn Break
  (Variables|Default|SetIsBroken true)
  (Variables|Default|SetMeal%20In%20Progress true)
  (Development|PrintString "BROKE")
  (Default|ToggleVisibility (Variables|Default|GetUI%20Reference) true)
  (Appearance|SetBrushfromTexture (Variables|/Game/UI/Progress_Bar_UI.Progress_Bar_UI_C|Getoutput_ingredient (Variables|Default|GetUI%20Reference)) "/Game/Textures/Sprites/New_Food_Sprites/UI_IngredientIceCreamBroken.UI_IngredientIceCreamBroken" false))

(fn GetOutput
  (bind _is_done (Variables|Default|GetIs%20Done))
  (if _is_done
    (return (Utilities|Struct|MakeST_Ingredient (Variables|Default|GetOutput%20Food) "NewEnumerator0" true) _is_done)
    (else
      (return (Utilities|Struct|MakeST_Ingredient "NewEnumerator20" "NewEnumerator0" false) _is_done))))

(fn ResetBoard
  (bind _returnvalue (Math|Random|RandomFloatinRange 0.0 101.0))
  (Development|PrintString "RESET")
  (Variables|Default|SetTimer 0.0)
  (if (Variables|Default|GetIsBroken)
    (Variables|Default|SetChance%20To%20Break 0.0)
    (Variables|Default|SetMeal%20In%20Progress false)
    (Variables|Default|SetIsBroken false)
    (Default|ToggleVisibility (Variables|Default|GetUI%20Reference) false)
    (else
      (Variables|Default|SetMeal%20In%20Progress false)
      (Variables|Default|SetIs%20Done false)
      (Default|ToggleVisibility (Variables|Default|GetUI%20Reference) false)
      (bind _output_get (Variables|Default|SetChance%20To%20Break (+ (Variables|Default|GetChance%20To%20Break) 15.0)))
      (Development|PrintString "RUNNING RANDo")
      (if (>= _output_get _returnvalue)
        (Development|PrintString "BREAK")
        (CallFunction|Break)
        (else
          (Development|PrintString (Utilities|String|ToString(Float) _returnvalue)))))))