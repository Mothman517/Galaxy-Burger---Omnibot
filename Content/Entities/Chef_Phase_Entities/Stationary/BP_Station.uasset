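; BP_Station is a stationary chef-phase station that the player chef can stand at to produce an ingredient.
; Its box overlap sets or clears the player's NearStation flag and CurrentStation reference.
; Helper functions map ingredient types to meshes, return OutputFood as a successful non-meal ingredient, and reset the board by destroying the spawn point's child components and setting MealInProgress.
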(event OnComponentBeginOverlap(Box)
  (params (OverlappedComponent :type Primitive%20Component%20Object%20Reference) (OtherActor :type Actor%20Object%20Reference) (OtherComp :type Primitive%20Component%20Object%20Reference) (OtherBodyIndex :type Integer) (bFromSweep :type Boolean) (SweepResult :type Hit%20Result%20Structure%20%28by%20ref%29))
  (bind _playerref (Variables|Default|GetPlayerRef))
  ;[0.15 0.15 0.15 0.5] collision
  (if (Actor|ActorHasTag OtherActor "Player")
    (Variables|/Game/PlayerControllers/Chef/Blueprints/BP_PlayerChef.BP_PlayerChef_C|SetNear%20Station _playerref true)
    (Variables|/Game/PlayerControllers/Chef/Blueprints/BP_PlayerChef.BP_PlayerChef_C|Setcurrent%20Station _playerref self)))

(event OnComponentEndOverlap(Box)
  (params (OverlappedComponent :type Primitive%20Component%20Object%20Reference) (OtherActor :type Actor%20Object%20Reference) (OtherComp :type Primitive%20Component%20Object%20Reference) (OtherBodyIndex :type Integer))
  (bind _playerref (Variables|Default|GetPlayerRef))
  ;[0.15 0.15 0.15 0.5] collision
  (if (Actor|ActorHasTag OtherActor "Player")
    (Variables|/Game/PlayerControllers/Chef/Blueprints/BP_PlayerChef.BP_PlayerChef_C|SetNear%20Station _playerref false)
    (Variables|/Game/PlayerControllers/Chef/Blueprints/BP_PlayerChef.BP_PlayerChef_C|Setcurrent%20Station _playerref 0)))

(event EventBeginPlay
  (bind _asbp_player_chef (Utilities|Casting|CastToBP_PlayerChef (Game|GetPlayerCharacter 0)))
  (Variables|Default|SetPlayerRef _asbp_player_chef))

(fn ConstructionScript)

(fn ResetBoard
  (bind _arrayelement (Utilities|Array|ReverseforEachLoop (Components|GetChildrenComponents (Variables|Default|GetIngredient%20Spawn%20Point) false))
    (:LoopBody
      (Components|DestroyComponent _arrayelement))
    (:Completed
      (Variables|Default|SetMeal%20In%20Progress true))))

(fn GetMesh
  (params (Ingredient :type Enum_CookingIngredients%20Enum :default "NewEnumerator0"))
  (switch Utilities|FlowControl|Switch|SwitchonEnum_CookingIngredients Ingredient
    (:NewEnumerator0
      (return "/Game/Models/cheese.cheese"))
    (:NewEnumerator1
      (return "/Game/Models/bottom_bun.bottom_bun"))
    (:NewEnumerator2
      (return "/Game/Models/patty.patty"))
    (:NewEnumerator3
      (return "/Game/Models/lettuce.lettuce"))
    (:NewEnumerator5
      (return "/Game/Models/tomatoes.tomatoes"))))

(fn GetOutput
  (return (Utilities|Struct|MakeST_Ingredient (Variables|Default|GetOutput%20Food) "NewEnumerator0" false) true))