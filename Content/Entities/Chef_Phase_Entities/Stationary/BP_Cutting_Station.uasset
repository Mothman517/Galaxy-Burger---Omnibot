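; Stationary cutting station that turns an eligible ingredient into its prepared form while the player holds interact nearby.
; StartChoppin validates the ingredient, maps it to an output via a switch and shows the progress bar widget, rotated toward the player camera on BeginPlay.
; Tick fills the timer while overlap permits cutting, optionally resetting on release.
; GetOutput returns the result once done, and ResetBoard clears the station.
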(event OnComponentBeginOverlap(Box)
  (params (OverlappedComponent :type Primitive%20Component%20Object%20Reference) (OtherActor :type Actor%20Object%20Reference) (OtherComp :type Primitive%20Component%20Object%20Reference) (OtherBodyIndex :type Integer) (bFromSweep :type Boolean) (SweepResult :type Hit%20Result%20Structure%20%28by%20ref%29))
  (if (Math|Boolean|ANDBoolean (Actor|ActorHasTag OtherActor "Player") (Variables|Default|GetMeal%20In%20Progress) (not (Variables|Default|GetIs%20Done)))
    (Variables|Default|SetCan%20Cut true)
    (Development|PrintString "CAN CUT")))

(event OnComponentEndOverlap(Box)
  (params (OverlappedComponent :type Primitive%20Component%20Object%20Reference) (OtherActor :type Actor%20Object%20Reference) (OtherComp :type Primitive%20Component%20Object%20Reference) (OtherBodyIndex :type Integer))
  (if (Actor|ActorHasTag OtherActor "Player")
    (Variables|Default|SetCan%20Cut false)))

(event Custom|Chop%20Food
  (params (Delta%20Time :type Float%20%28double-precision%29)))

(event EventBeginPlay
  (bind _playerref (Variables|Default|GetPlayerRef))
  (bind _widget (Variables|Default|GetWidget))
  (bind _returnvalue (Transformation|GetWorldLocation _widget))
  (bind _camposition (Variables|/Game/PlayerControllers/Chef/Blueprints/BP_PlayerChef.BP_PlayerChef_C|GetCamPosition _playerref))
  (bind _returnvalue_2 (Math|Rotator|FindLookatRotation _returnvalue _camposition))
  (|CallParentFunction)
  (Transformation|SetWorldRotation _widget (Math|Rotator|MakeRotator 0.0 (.pitch _returnvalue_2) (.yaw _returnvalue_2)) false false)
  (bind _asprogress_bar_ui (Utilities|Casting|CastToProgress_Bar_UI (UserInterface|GetWidget (Variables|Default|GetWidget))))
  (Variables|Default|SetUI%20Reference _asprogress_bar_ui))

(event EventTick
  (params (DeltaSeconds :type Float%20%28single-precision%29))
  (if (Variables|Default|GetCan%20Cut)
    (if (Variables|/Game/PlayerControllers/Chef/Blueprints/BP_PlayerChef.BP_PlayerChef_C|GetHolding%20Interact (Variables|Default|GetPlayerRef))
      (Variables|Default|SetTimer (+ DeltaSeconds (Variables|Default|GetTimer)))
      (if (>= (Variables|Default|GetTimer) (Variables|Default|GetTime%20To%20Prepare)) :!label _label
        (Variables|Default|SetIs%20Done true)
        (Variables|Default|SetCan%20Cut false))
      (Default|SetPercent (Variables|Default|GetUI%20Reference) (/ (Variables|Default|GetTimer) (Variables|Default|GetTime%20To%20Prepare)))
      (elif (and (Variables|Default|GetReset%20If%20Released) (not (Variables|Default|GetIs%20Done)))
        (Variables|Default|SetTimer 0.0)
        (goto _label)))))

(fn ConstructionScript
  (|CallParentFunction))

(fn StartChoppin
  (params (Ingredient :type Enum_CookingIngredients%20Enum :default "NewEnumerator0"))
  (if (Utilities|Array|ContainsItem (Variables|Default|GetElgible%20Ingredients) Ingredient)
    (Variables|Default|SetInput%20Food Ingredient)
    (CallFunction|SetOutput)
    (bind _output_get (Variables|Default|SetMeal%20In%20Progress true))
    (Development|PrintString "chopped")
    (Default|ToggleVisibility (Variables|Default|GetUI%20Reference) true)
    (Variables|Default|SetCan%20Cut true)
    (return _output_get)
    (else
      (Development|PrintString "Nuh uh")
      (return false))))

(fn GetOutput
  (bind _is_done (Variables|Default|GetIs%20Done))
  (if _is_done
    (return (Utilities|Struct|MakeST_Ingredient (Variables|Default|GetOutput%20Food) "NewEnumerator0" false) _is_done)
    (else
      (return (Utilities|Struct|MakeST_Ingredient "NewEnumerator20" "NewEnumerator0" false) _is_done))))

(fn SetOutput
  (switch Utilities|FlowControl|Switch|SwitchonEnum_CookingIngredients (Variables|Default|GetInput%20Food)
    (:NewEnumerator21
      (bind _output_get (Variables|Default|SetOutput%20Food "NewEnumerator2"))
      (Default|SetImage (Variables|Default|GetUI%20Reference) _output_get :!label _label))
    (:NewEnumerator5
      (Variables|Default|SetOutput%20Food "NewEnumerator17")
      (goto _label))
    (:NewEnumerator6
      (Variables|Default|SetOutput%20Food "NewEnumerator18")
      (goto _label))
    (:NewEnumerator18
      (Variables|Default|SetOutput%20Food "NewEnumerator13"))
    (:NewEnumerator7
      (Variables|Default|SetOutput%20Food "NewEnumerator14")
      (goto _label))
    (:NewEnumerator14
      (Variables|Default|SetOutput%20Food "NewEnumerator19"))))

(fn ResetBoard
  (Variables|Default|SetTimer 0.0)
  (Variables|Default|SetInput%20Food "NewEnumerator20")
  (Variables|Default|SetOutput%20Food "NewEnumerator20")
  (Variables|Default|SetMeal%20In%20Progress false)
  (Variables|Default|SetIs%20Done false)
  (Default|ToggleVisibility (Variables|Default|GetUI%20Reference) false))