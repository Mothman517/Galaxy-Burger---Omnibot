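; BP_Blender is a stationary recipe station in the chef phase that combines needed ingredients into an output food pickup.
; A trigger box registers it on the player chef as the current blender while in range.
; IsPartOfRecipe marks accepted ingredients, spawning the output pickup and resetting once all are in.
; Paper sprites built at runtime show the recipe, green when acquired, yawed toward the player's camera position on each rebuild.
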(event OnComponentBeginOverlap(Box)
  (params (OverlappedComponent :type Primitive%20Component%20Object%20Reference) (OtherActor :type Actor%20Object%20Reference) (OtherComp :type Primitive%20Component%20Object%20Reference) (OtherBodyIndex :type Integer) (bFromSweep :type Boolean) (SweepResult :type Hit%20Result%20Structure%20%28by%20ref%29))
  (bind _playerref (Variables|Default|GetPlayerRef))
  ;[0.15 0.15 0.15 0.5] Toggle Collision
  (if (Actor|ActorHasTag OtherActor "Player")
    (Variables|/Game/PlayerControllers/Chef/Blueprints/BP_PlayerChef.BP_PlayerChef_C|SetNear%20Blender _playerref true)
    (Variables|/Game/PlayerControllers/Chef/Blueprints/BP_PlayerChef.BP_PlayerChef_C|SetcurrentBlender _playerref self)))

(event OnComponentEndOverlap(Box)
  (params (OverlappedComponent :type Primitive%20Component%20Object%20Reference) (OtherActor :type Actor%20Object%20Reference) (OtherComp :type Primitive%20Component%20Object%20Reference) (OtherBodyIndex :type Integer))
  (bind _playerref (Variables|Default|GetPlayerRef))
  ;[0.15 0.15 0.15 0.5] Toggle Collision
  (if (Actor|ActorHasTag OtherActor "Player")
    (Variables|/Game/PlayerControllers/Chef/Blueprints/BP_PlayerChef.BP_PlayerChef_C|SetNear%20Blender _playerref false)
    (Variables|/Game/PlayerControllers/Chef/Blueprints/BP_PlayerChef.BP_PlayerChef_C|SetcurrentBlender _playerref 0)))

(event EventBeginPlay
  ;[0.15 0.15 0.15 0.5] Initialize
  (Utilities|Array|Resize (Variables|Default|GetAcquired%20Ingredients) (Utilities|Array|Length (Variables|Default|GetNeeded%20Ingredients)))
  (bind _asbp_player_chef (Utilities|Casting|CastToBP_PlayerChef (Game|GetPlayerCharacter 0)))
  (Variables|Default|SetPlayerRef _asbp_player_chef)
  (CallFunction|UpdatePaperSprites))

(fn ConstructionScript)

(fn UpdatePaperSprites
  ;[0.15 0.15 0.15 0.5] Set Sprite
  (Variables|Default|SetCurrent%20Vector%20Modifier "0, 0, 0")
  (LocalVariables|SettempPaperSprite 0)
  (for (_array_element _array_index) (Variables|Default|GetNeeded%20Ingredients)
    (bind _returnvalue (AddComponent|AddPaperSpriteComponent false))
    (Transformation|AttachComponentToComponent _returnvalue (Variables|Default|GetspritePivot) "None" "KeepRelative" "KeepRelative" "KeepRelative" true)
    (Utilities|Array|Add (Variables|Default|GetspriteArray) _returnvalue)
    (switch Utilities|FlowControl|Switch|SwitchonEnum_CookingIngredients _array_element
      (:NewEnumerator0
        (LocalVariables|SettempPaperSprite "/Game/Sprites/cheese_testsprite_Sprite.cheese_testsprite_Sprite"))
      (:NewEnumerator1
        (LocalVariables|SettempPaperSprite "/Game/Sprites/buns_testsprite_Sprite.buns_testsprite_Sprite"))
      (:NewEnumerator2
        (LocalVariables|SettempPaperSprite "/Game/Sprites/steak_testsprite_Sprite.steak_testsprite_Sprite"))
      (:NewEnumerator3
        (LocalVariables|SettempPaperSprite "/Game/Sprites/burger_testsprite_Sprite.burger_testsprite_Sprite")))
    (Rendering|Components|Sprite|SetSprite _returnvalue (LocalVariables|GettempPaperSprite))
    (if (Utilities|Array|Get(acopy) (Variables|Default|GetAcquired%20Ingredients) _array_index)
      (Sprite|SetSpriteColor _returnvalue "(R=0.000000,G=1.000000,B=0.000000,A=1.000000)")
      (else
        (Sprite|SetSpriteColor _returnvalue "(R=1.000000,G=1.000000,B=1.000000,A=1.000000)")))
    (bind _output_get (Variables|Default|SetCurrent%20Vector%20Modifier (+ (Variables|Default|GetCurrent%20Vector%20Modifier) (Variables|Default|GetSprite%20Distance))))
    (Transformation|SetRelativeLocation _returnvalue _output_get false false)
    ;[0.15 0.15 0.15 0.5] Billboard
    (bind _asbp_player_chef (Utilities|Casting|CastToBP_PlayerChef (Game|GetPlayerCharacter 0)))
    (Transformation|SetWorldRotation _returnvalue (Math|Rotator|MakeRotator 0.0 0.0 (+ (.Yaw (Math|Rotator|BreakRotator (Math|Rotator|FindLookatRotation (Variables|/Game/PlayerControllers/Chef/Blueprints/BP_PlayerChef.BP_PlayerChef_C|GetCamPosition _asbp_player_chef) (Transformation|GetWorldLocation _returnvalue)))) -9e+01)) false false)))

(fn ClearPaperSprites
  (bind _spritearray (Variables|Default|GetspriteArray))
  (bind _arrayelement (Utilities|Array|ReverseforEachLoop _spritearray)
    (:LoopBody
      (Components|DestroyComponent _arrayelement))
    (:Completed
      (Utilities|Array|Resize _spritearray 0))))

(fn IsPartOfRecipe
  (params (Ingredient :type Enum_CookingIngredients%20Enum :default "NewEnumerator0"))
  (bind _acquired_ingredients (Variables|Default|GetAcquired%20Ingredients))
  (bind _needed_ingredients (Variables|Default|GetNeeded%20Ingredients))
  (bind _returnvalue (Utilities|Array|FindItem _needed_ingredients Ingredient))
  (if (Utilities|Array|ContainsItem _needed_ingredients Ingredient)
    (if (not (Utilities|Array|Get(acopy) _acquired_ingredients _returnvalue))
      (Utilities|Array|SetArrayElem _acquired_ingredients _returnvalue true)
      (CallFunction|ClearPaperSprites)
      (CallFunction|UpdatePaperSprites)
      (bind _is_complete (CallFunction|IsRecipeDone))
      (if _is_complete
        (CallFunction|SpawnOutput))
      (return true)
      (else
        _)))
  (return false))

(fn IsRecipeDone
  (bind _array_element (Utilities|Array|ForEachLoopwithBreak (Variables|Default|GetAcquired%20Ingredients))
    (:LoopBody
      (if (not _array_element)
        (return false)))
    (:Completed
      (return true))))

(fn SpawnOutput
  (bind _acquired_ingredients (Variables|Default|GetAcquired%20Ingredients))
  (bind _outputspawnpoint (Variables|Default|GetoutputSpawnpoint))
  (bind _returnvalue (Transformation|GetWorldTransform _outputspawnpoint))
  (bind _array_index (Utilities|Array|ForEachLoopwithBreak _acquired_ingredients)
    (:LoopBody
      (Utilities|Array|SetArrayElem _acquired_ingredients _array_index false))
    (:Completed
      (Development|PrintString (Utilities|String|ToString(Transform) _returnvalue))
      (Game|SpawnActorfromClass "/Game/Entities/Chef_Phase_Entities/FoodItems/BP_BaseIngredientPickup.BP_BaseIngredientPickup_C" _returnvalue "Undefined" "MultiplyWithRoot" 0 (Variables|Default|GetOutputFood) 0)
      (CallFunction|ClearPaperSprites)
      (CallFunction|UpdatePaperSprites))))