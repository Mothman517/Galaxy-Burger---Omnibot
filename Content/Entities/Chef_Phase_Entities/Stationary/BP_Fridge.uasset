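; Stationary fridge for the chef phase that supplies a selected base ingredient to the player.
; On BeginPlay it gets the eligible ingredient list from BP_GameData on the game instance and creates a Fridge_UI widget with that inventory.
; When IsDone is set, GetOutput calls InteractWithFridge on the player and returns the ingredient at SelectedIndex as a non-meal; otherwise it reports failure.
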(event EventBeginPlay
  (|CallParentFunction)
  (bind _asbp_game_data (Utilities|Casting|CastToBP_GameData (Game|GetGameInstance)))
  (bind _list (Default|CreateFridgeList _asbp_game_data))
  (bind _output_get (Variables|Default|SetElgible%20Ingredients _list))
  (bind _returnvalue (UserInterface|CreateWidget "/Game/UI/Fridge_UI.Fridge_UI_C" 0 _output_get))
  (Variables|Default|SetFridge%20UI%20Ref _returnvalue))

(event Collision|EventActorBeginOverlap
  (params (OtherActor :type Actor%20Object%20Reference)))

(event EventTick
  (params (DeltaSeconds :type Float%20%28single-precision%29)))

(fn ConstructionScript
  (|CallParentFunction))

(fn GetOutput
  (if (Variables|Default|GetIs%20Done)
    (Default|InteractwithFridge (Variables|Default|GetPlayerRef))
    (return (Utilities|Struct|MakeST_Ingredient (Utilities|Array|Get(acopy) (Variables|Default|GetElgible%20Ingredients) (Variables|Default|GetSelected%20Index)) "NewEnumerator20" false) true)
    (else
      (return "" false))))