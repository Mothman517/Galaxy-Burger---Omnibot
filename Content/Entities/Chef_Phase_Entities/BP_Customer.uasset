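; BP_Customer is a Chef-phase entity that the player can harvest for an item and that can leave a corpse.
; BeginPlay configures its HarvestableComponent with the milked item and harvest flags, then caches the BP_PlayerHunter reference.
; Sphere overlaps set or clear that component as the player's closest harvestable, with debug prints.
; LeaveCorpse replaces the customer with a BP_Corpse whose harvestable resource is the customer's ItemDrop.
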(event OnComponentBeginOverlap(Sphere)
  (params (OverlappedComponent :type Primitive%20Component%20Object%20Reference) (OtherActor :type Actor%20Object%20Reference) (OtherComp :type Primitive%20Component%20Object%20Reference) (OtherBodyIndex :type Integer) (bFromSweep :type Boolean) (SweepResult :type Hit%20Result%20Structure%20%28by%20ref%29))
  ;[0.15 0.15 0.15 0.5] Collision Detection Toggles
  (if (Actor|ActorHasTag OtherActor "Player")
    (Variables|/Game/PlayerControllers/Hunter/Blueprints/BP_PlayerHunter.BP_PlayerHunter_C|SetClosest%20Harvestable (Variables|Default|GetPlayerRef) (Variables|Default|GetHarvestableComponent))
    (Development|PrintString "IN")))

(event OnComponentEndOverlap(Sphere)
  (params (OverlappedComponent :type Primitive%20Component%20Object%20Reference) (OtherActor :type Actor%20Object%20Reference) (OtherComp :type Primitive%20Component%20Object%20Reference) (OtherBodyIndex :type Integer))
  ;[0.15 0.15 0.15 0.5] Collision Detection Toggles
  (if (Actor|ActorHasTag OtherActor "Player")
    (Variables|/Game/PlayerControllers/Hunter/Blueprints/BP_PlayerHunter.BP_PlayerHunter_C|SetClosest%20Harvestable (Variables|Default|GetPlayerRef) 0)
    (Development|PrintString "OUT")))

(event EventBeginPlay
  (bind _harvestablecomponent (Variables|Default|GetHarvestableComponent))
  ;[0.15 0.15 0.15 0.5] Set up Harvestable Component
  (|CallParentFunction)
  (Default|SetVariables _harvestablecomponent (Variables|Default|GetMilkedItem) (Variables|Default|GetHas%20Been%20Harvested) (Variables|Default|GetDestroyOnHarvest))
  (Variables|/Game/Entities/Hunter_Phase_Entities/Components/HarvestableComponent.HarvestableComponent_C|SetObtainableResource _harvestablecomponent (Variables|Default|GetMilkedItem))
  (bind _asbp_player_hunter (Utilities|Casting|CastToBP_PlayerHunter (Game|GetPlayerCharacter 0)))
  (Variables|Default|SetPlayerRef _asbp_player_hunter))

(event Collision|EventActorBeginOverlap
  (params (OtherActor :type Actor%20Object%20Reference)))

(event EventTick
  (params (DeltaSeconds :type Float%20%28single-precision%29))
  (|CallParentFunction DeltaSeconds) ; This node is disabled and will not be called.\nDrag off pins to build functionality.
)

(fn ConstructionScript
  (|CallParentFunction))

(fn LeaveCorpse
  (bind _returnvalue (Game|SpawnActorfromClass "/Game/Entities/Hunter_Phase_Entities/Animals/BP_Corpse.BP_Corpse_C" (Transformation|GetActorTransform) "AdjustIfPossibleButAlwaysSpawn" "MultiplyWithRoot" 0 0))
  (Variables|/Game/Entities/Hunter_Phase_Entities/Components/HarvestableComponent.HarvestableComponent_C|SetObtainableResource (Variables|/Game/Entities/Hunter_Phase_Entities/Animals/BP_Corpse.BP_Corpse_C|GetHarvestableComponent _returnvalue) (Variables|Default|GetItemDrop))
  (Actor|DestroyActor))