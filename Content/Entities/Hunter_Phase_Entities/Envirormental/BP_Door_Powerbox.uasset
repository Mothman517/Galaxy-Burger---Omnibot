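; BP_Door_Powerbox is an environmental power box for the hunter phase that opens a gate and spawns animals when toggled.
; It extends a parent's ToggleBox event, acting only while IsBroken is false.
; A successful toggle runs the parent logic, plays a power sound, opens the referenced Gate, then calls SpawnAnimal on each entry in AnimalsIsSpawn.
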(event Collision|EventActorBeginOverlap
  (params (OtherActor :type Actor%20Object%20Reference))
  (|CallParentFunction OtherActor) ; This node is disabled and will not be called.\nDrag off pins to build functionality.
)

(event EventTick
  (params (DeltaSeconds :type Float%20%28single-precision%29))
  (|CallParentFunction DeltaSeconds) ; This node is disabled and will not be called.\nDrag off pins to build functionality.
)

(event EventToggleBox
  (if (not (Variables|Default|GetIs%20Broken))
    (|CallParentFunction)
    (Audio|PlaySound2D "/Game/Materials/MUSIC/Power_SFX_Cue.Power_SFX_Cue" 0.6 1.0 2.0 0 0)
    (Default|EventOpenGate (Variables|Default|GetGate))
    (for _array_element (Variables|Default|GetAnimals%20Is%20Spawn)
      (Default|SpawnAnimal _array_element))))

(fn ConstructionScript
  (|CallParentFunction))