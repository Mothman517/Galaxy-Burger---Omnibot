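; BP_Gate is an environmental gate actor for the hunter phase that slides between a closed and an open position.
; It records its starting location as the closed position on BeginPlay.
; OpenGate plays a timeline that lerps the actor to OpenPosition, and CloseGate reverses the same timeline to move it back.
; Debug prints report closing and the timeline direction when movement finishes.
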(event Custom|Event%20Open%20Gate
  (bind (_direction _alpha) (Timeline|AlphaTimeline Play)
    (:Update
      (Transformation|SetActorLocation (Math|Vector|Lerp(Vector) (Variables|Default|GetClosed%20Position) (Variables|Default|GetOpen%20Position) _alpha) false false))
    (:Finished
      (Development|PrintString (Utilities|String|EnumtoString _direction)))))

(event Custom|Event%20Close%20Gate
  (Development|PrintString "closing gate")
  (bind (_direction _alpha) (Timeline|AlphaTimeline Reverse)
    (:Update
      (Transformation|SetActorLocation (Math|Vector|Lerp(Vector) (Variables|Default|GetClosed%20Position) (Variables|Default|GetOpen%20Position) _alpha) false false))
    (:Finished
      (Development|PrintString (Utilities|String|EnumtoString _direction)))))

(event EventBeginPlay
  (Variables|Default|SetClosed%20Position (Transformation|GetActorLocation self)))

(fn ConstructionScript)