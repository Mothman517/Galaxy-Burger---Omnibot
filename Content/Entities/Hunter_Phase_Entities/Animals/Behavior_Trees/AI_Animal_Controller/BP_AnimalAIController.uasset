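; AI controller for huntable animals that runs their behavior tree and switches them between normal and fleeing speed.
; On possession it starts BT_Animal_Tree, casts the pawn to Test_Animal and caches its movement speed as the normal speed.
; EnableIsRunningAway sets the running-away blackboard flag, raises walk speed to sprint and writes a random tick count from the animal's RunAwayTicks range.
; SlowDown restores the cached speed, leaving the blackboard untouched.
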(event Custom|Enable%20IsRunningAway
  (bind _blackboard (Variables|Default|GetBlackboard))
  (bind _animalref (Variables|Default|GetAnimalRef))
  (bind _run_away_ticks (Variables|/Game/Entities/Hunter_Phase_Entities/Animals/Test_Animal.Test_Animal_C|GetRun%20Away%20Ticks _animalref))
  (AI|Components|Blackboard|SetValueasBool _blackboard (Variables|Default|GetRunning%20Away%20Key%20Name) true)
  (Variables|/Script/Engine.CharacterMovementComponent|SetMaxWalkSpeed (Variables|/Script/Engine.Character|GetCharacterMovement _animalref) (Variables|Default|GetSprint%20Walk%20Speed))
  (Class|BlackboardComponent|SetValueasInt _blackboard (Variables|Default|GetTicks%20Key%20Name) (Math|Random|RandomIntegerinRange (Utilities|Array|Get(acopy) _run_away_ticks) (Utilities|Array|Get(acopy) _run_away_ticks 1))))

(event Custom|Slow%20Down
  (Variables|/Script/Engine.CharacterMovementComponent|SetMaxWalkSpeed (Variables|/Script/Engine.Character|GetCharacterMovement (Variables|Default|GetAnimalRef)) (Variables|Default|GetNormal%20Walk%20Speed)))

(event EventPossess
  (params (PossessedPawn :type Pawn%20Object%20Reference))
  (AI|RunBehaviorTree "/Game/Entities/Hunter_Phase_Entities/Animals/Behavior_Trees/AI_Animal_Controller/BT_Animal_Tree.BT_Animal_Tree")
  (bind _astest_animal (Utilities|Casting|CastToTest_Animal PossessedPawn))
  (bind _output_get (Variables|Default|SetAnimalRef _astest_animal))
  (Variables|Default|SetNormal%20Walk%20Speed (Class|MovementComponent|GetMaxSpeed (Variables|/Script/Engine.Character|GetCharacterMovement _output_get))))

(fn ConstructionScript)