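; BP_GameData holds day-based game progression for a food-themed game: the day counter, money quota, score, ingredient lists and fridge lists.
; CreateList and CreateFridgeList switch on Day to return growing item sets, with randomized ingredient quantities that scale with Day in the default case.
; Increment functions advance the day and quota.
; Scoring functions compare tips to DailyQuota and ingredient counts to that day's IngredientLists entry, then update Score.
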(fn CreateList
  (bind _returnvalue (Math|Random|RandomIntegerinRange 2 3))
  (bind _returnvalue_2 (Math|Random|RandomIntegerinRange 1 2))
  (bind _returnvalue_3 (Math|Random|RandomIntegerinRange 2 5))
  (bind _returnvalue_4 (Math|Random|RandomIntegerinRange 1 2))
  (bind _day (Variables|Default|GetDay))
  (bind _day_2 (Variables|Default|GetDay))
  (bind _returnvalue_5 (* _returnvalue_4 _returnvalue))
  (bind _returnvalue_6 (* _returnvalue_2 _returnvalue_3))
  (Development|PrintText (Utilities|Text|ToText(Integer) _day))
  (switch int _day
    (:Default
      (return (Utilities|Struct|MakeST_IngredientList (Utilities|Array|MakeArray "NewEnumerator0" "NewEnumerator1" "NewEnumerator2" "NewEnumerator5" "NewEnumerator6" "NewEnumerator13" "NewEnumerator12") (Utilities|Array|MakeArray (+ _day_2 (Math|Random|RandomIntegerinRange -2 2)) (+ _day_2 (Math|Random|RandomIntegerinRange -2 2)) (+ _day_2 (Math|Random|RandomIntegerinRange -2 2)) (+ _day_2 (Math|Random|RandomIntegerinRange -2 2)) (+ _day_2 (Math|Random|RandomIntegerinRange -2 2)) (+ _day_2 (Math|Random|RandomIntegerinRange -2 2)) (+ _day_2 (Math|Random|RandomIntegerinRange -2 2))))))
    (:0
      (return (Utilities|Struct|MakeST_IngredientList (Utilities|Array|MakeArray "NewEnumerator2" "NewEnumerator1" "NewEnumerator0") (Utilities|Array|MakeArray _returnvalue_5 _returnvalue_5 _returnvalue_6))))
    (:1
      (return (Utilities|Struct|MakeST_IngredientList (Utilities|Array|MakeArray "NewEnumerator2" "NewEnumerator1" "NewEnumerator0" "NewEnumerator5") (Utilities|Array|MakeArray _returnvalue_5 _returnvalue_5 _returnvalue_6 _returnvalue_6))))
    (:2
      (return (Utilities|Struct|MakeST_IngredientList (Utilities|Array|MakeArray "NewEnumerator2" "NewEnumerator1" "NewEnumerator0" "NewEnumerator5" "NewEnumerator6") (Utilities|Array|MakeArray _returnvalue_5 _returnvalue_5 _returnvalue_6 _returnvalue_6 _returnvalue_6))))
    (:3
      (return (Utilities|Struct|MakeST_IngredientList (Utilities|Array|MakeArray "NewEnumerator0" "NewEnumerator1" "NewEnumerator2" "NewEnumerator6" "NewEnumerator5" "NewEnumerator13") (Utilities|Array|MakeArray _returnvalue_5 _returnvalue_5 _returnvalue_6 _returnvalue_6 _returnvalue_6 _returnvalue_5))))))

(fn PrintList
  (params (WhichDay :type Integer))
  (bind _ingredientlists (Variables|Default|GetIngredientLists))
  (bind _output (Utilities|Array|Get(acopy) _ingredientlists WhichDay))
  (bind (_typelist _quantitylist) (Utilities|Struct|BreakST_IngredientList _output))
  (for (_array_element _array_index) _typelist
    (Development|PrintString (Utilities|String|Append (Utilities|String|EnumtoString _array_element) (Utilities|String|Append ", " (Utilities|String|ToString(Integer) (Utilities|Array|Get(acopy) _quantitylist _array_index)))))))

(fn CreateFridgeList
  (switch int (Variables|Default|GetDay)
    (:Default
      (return (Utilities|Array|MakeArray "NewEnumerator0" "NewEnumerator1" "NewEnumerator21" "NewEnumerator3" "NewEnumerator5" "NewEnumerator6" "NewEnumerator7" "NewEnumerator15" "NewEnumerator22")))
    (:0
      (return (Utilities|Array|MakeArray "NewEnumerator0" "NewEnumerator1" "NewEnumerator21" "NewEnumerator3" "NewEnumerator5")))
    (:1
      (return (Utilities|Array|MakeArray "NewEnumerator0" "NewEnumerator1" "NewEnumerator21" "NewEnumerator3" "NewEnumerator5")))
    (:2
      (return (Utilities|Array|MakeArray "NewEnumerator0" "NewEnumerator1" "NewEnumerator21" "NewEnumerator3" "NewEnumerator5" "NewEnumerator6")))
    (:3
      (return (Utilities|Array|MakeArray "NewEnumerator0" "NewEnumerator1" "NewEnumerator21" "NewEnumerator3" "NewEnumerator5" "NewEnumerator6" "NewEnumerator7")))
    (:4
      (return (Utilities|Array|MakeArray "NewEnumerator0" "NewEnumerator1" "NewEnumerator21" "NewEnumerator3" "NewEnumerator5" "NewEnumerator6" "NewEnumerator7" "NewEnumerator15")))
    (:5
      (return (Utilities|Array|MakeArray "NewEnumerator0" "NewEnumerator1" "NewEnumerator21" "NewEnumerator3" "NewEnumerator5" "NewEnumerator6" "NewEnumerator7" "NewEnumerator20" "NewEnumerator22")))))

(fn IncrementDay
  (Variables|Default|SetDay (+ (Variables|Default|GetDay) 1)))

(fn IncrementQuota
  (Variables|Default|SetDaily%20Quota (+ (Variables|Default|GetDaily%20Quota) 12.0)))

(fn AddtoScoreViaMoney
  (params (Tips :type Float%20%28double-precision%29))
  (Development|PrintString (Utilities|String|ToString(Float) Tips))
  (bind _output_get (LocalVariables|SetDaily%20Score (Math|Float|Truncate (* (- Tips (Variables|Default|GetDaily%20Quota)) 1e+01))))
  (Variables|Default|SetScore (+ (* _output_get 100) (Variables|Default|GetScore)))
  (return (* _output_get 100)))

(fn AddtoScoreViaIngredient
  (params (Ingredients :type Array%20of%20Integers))
  (Development|PrintString "TEST CAST")
  (for (_array_element _array_index) Ingredients
    (LocalVariables|SetDaily%20Score (+ (LocalVariables|GetTotal%20Score) (* (- _array_element (Utilities|Array|Get(acopy) (.quantitylist (Utilities|Array|Get(acopy) (Variables|Default|GetIngredientLists) (Variables|Default|GetDay))) _array_index)) 30))))
  (bind _output_get (Variables|Default|SetScore (* (+ (LocalVariables|GetDaily%20Score) (Variables|Default|GetScore)) 100)))
  (return _output_get))